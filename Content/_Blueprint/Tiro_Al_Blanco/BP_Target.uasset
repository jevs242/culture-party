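; BP_Target is a target for the Tiro_Al_Blanco shooting game that awards points when hit by a bullet.
; An overlap on its collision component casts the other actor to BP_Bala_Tiro_Al_Blanco, stores it and fires the The_Target event.
; That event spawns an emitter and sound at the target, calls SumaDePuntos on the bullet's Character reference, then destroys the target.
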(event `The_Target`
  (bind _returnvalue (`self.K2_GetActorLocation`))
  ;[1 0.8179 0.01812] Target
  (`GameplayStatics.SpawnEmitterAtLocation` null _returnvalue)
  (`GameplayStatics.PlaySoundAtLocation` null _returnvalue (struct) 1.0 1.0 0.0 null null null)
  (`/Game/_Blueprint/Tiro_Al_Blanco/Tiro_Al_Blanco_Character.SumaDePuntos` (`/Game/_Blueprint/Tiro_Al_Blanco/BP_Bala_Tiro_Al_Blanco.Character` (`self.As BP Bala Tiro Al Blanco`)))
  (`self.K2_DestroyActor`))

(event `self.TargetCollision.OnComponentBeginOverlap`
  (params (OverlappedComponent :type "PrimitiveComponent Object Reference") (OtherActor :type "Actor Object Reference") (OtherComp :type "PrimitiveComponent Object Reference") (OtherBodyIndex :type Integer) (bFromSweep :type Boolean) (SweepResult :type "HitResult Structure (by ref)"))
  ;[1 0.8179 0.01812] Target
  (bind _asbp_bala_tiro_al_blanco (cast `/Game/_Blueprint/Tiro_Al_Blanco/BP_Bala_Tiro_Al_Blanco` OtherActor))
  (set `self.As BP Bala Tiro Al Blanco` _asbp_bala_tiro_al_blanco)
  (`self.The_Target`))

(fn `UserConstructionScript`)