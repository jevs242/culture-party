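; Bottle-flip minigame Blueprint where Space stops a swinging rotation arm and launches the bottle toss.
; The captured angle sets the random-roll range through threshold checks, with higher angles up to 45 improving the odds.
; A timeline moves the scene component, then success adds a point while failure lets the mesh fall with physics.
; After a delay, transforms reset and the swing restarts until three points are scored.
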(event `self.ReceiveBeginPlay`
  (set `self.Scene_LocationRotation` (`SceneComponent.K2_GetComponentToWorld` (`self.Scene`)))
  (set `self.Mesh_LocationRotation` (`SceneComponent.K2_GetComponentToWorld` (`self.StaticMesh`)))
  (bind (_direction _float) (`Timeline|Rotation Arm` :!label _label)
    (:`Update`
      (`SceneComponent.K2_SetWorldRotation` (`self.Scene`) (`KismetMathLibrary.MakeRotator` 0.0 _float) false false))))

(event `BeginRotation`
  (`SceneComponent.K2_AttachToComponent` (`self.StaticMesh`) (`self.Scene`) "None" "KeepWorld" "KeepWorld" "KeepWorld" false)
  (goto _label :!via `PlayFromStart`))

(event `Stop`
  (set `self.Angle` (stale `self.ReceiveBeginPlay` _float))
  (goto _label :!via `Stop`))

(event `Set Points`
  (params (Points :type Integer))
  (set `self.Points` Points))

(event `Key|SpaceBar`
  (params (Key :type "Key Structure"))
  (bind _staticmesh (`self.StaticMesh`))
  (bind (_returnvalue_x _returnvalue_y _returnvalue_z) (`KismetMathLibrary.BreakVector` (`SceneComponent.K2_GetComponentLocation` (`self.Scene`))))
  (:`Pressed`
    (if (`self.InputActivate`)
      (set `self.InputActivate` false)
      (`self.Stop`)
      (if (<= (`self.Angle`) 0.0)
        (set `self.MaxNumber` 0)
        (bind (_direction _newtrack_0 _newtrack_1) (`Timeline|Timeline_0` :!via `PlayFromStart` :!label _label_2)
          (:`Update`
            (`SceneComponent.K2_SetWorldLocationAndRotation` (`self.Scene`) (`KismetMathLibrary.MakeVector` (+ _newtrack_1 _returnvalue_x) _returnvalue_y (- _returnvalue_z _newtrack_1)) (`KismetMathLibrary.MakeRotator` 0.0 _newtrack_0) false false))
          (:`Finished`
            (if (== 0 (`KismetMathLibrary.RandomIntegerInRange` 0 (`self.MaxNumber`)))
              (bind _result (`/Engine/EditorBlueprintResources/StandardMacros.IncrementInt` (`self.Points`))
                (:`  `
                  (`self.Set Points` _result)))
              (else
                (`PrimitiveComponent.SetSimulatePhysics` _staticmesh true)))
            (`KismetSystemLibrary.Delay` 4.0)
            (`PrimitiveComponent.SetSimulatePhysics` _staticmesh false)
            (`SceneComponent.K2_SetWorldTransform` (`self.Scene`) (`self.Scene_LocationRotation`) false false)
            (`SceneComponent.K2_SetWorldTransform` (`self.StaticMesh`) (`self.Mesh_LocationRotation`) false false)
            (`KismetSystemLibrary.Delay` 1.0)
            (if (<= (`self.Points`) 2)
              (set `self.InputActivate` true)
              (`self.BeginRotation`))))
        (elif (<= (`self.Angle`) 0.0)
          (set `self.MaxNumber` 0)
          (goto _label_2 :!via `PlayFromStart`)
          (elif (<= (`self.Angle`) 0.0)
            (set `self.MaxNumber` 0)
            (goto _label_2 :!via `PlayFromStart`)
            (elif (<= (`self.Angle`) 0.0)
              (set `self.MaxNumber` 0)
              (goto _label_2 :!via `PlayFromStart`)
              (elif (<= (`self.Angle`) 0.0)
                (set `self.MaxNumber` 0)
                (goto _label_2 :!via `PlayFromStart`)
                (elif (<= (`self.Angle`) 0.0)
                  (set `self.MaxNumber` 0)
                  (goto _label_2 :!via `PlayFromStart`))))))))))

(fn `UserConstructionScript`)