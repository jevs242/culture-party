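; Lobby actor, named as the lobby camera, that opens the lobby menu when play begins.
; With authority, it first copies MaxPlayer from BP_PartyGameInstance.
; On both authority and remote, it then creates WBP_MenuLobby for player controller 0, passes in MaxPlayer, adds it to the player screen and shows the mouse cursor.
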(event `self.ReceiveBeginPlay`
  (bind _returnvalue (`GameplayStatics.GetPlayerController` 0))
  (`/Engine/EditorBlueprintResources/ActorMacros.Switch Has Authority`
    (:`Authority`
      (`self.Set Max Player Server`))
    (:`Remote`
      _))
  (bind _returnvalue_2 (`|CreateWidget` "/Game/_Blueprint/_Menu/WBP_MenuLobby.WBP_MenuLobby_C" _returnvalue (`self.MaxPlayer`)))
  (`UserWidget.AddToPlayerScreen` _returnvalue_2 0)
  (set `PlayerController.bShowMouseCursor` true _returnvalue))

(event `Set Max Player Server`
  (bind _asbp_party_game_instance (cast `/Game/_Blueprint/_Base/BP_PartyGameInstance` (`GameplayStatics.GetGameInstance`)))
  (set `self.MaxPlayer` (`/Game/_Blueprint/_Base/BP_PartyGameInstance.MaxPlayer` _asbp_party_game_instance)))

(fn `UserConstructionScript`)