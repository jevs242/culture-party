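; BP_Block is a block actor in the Party content that displays a type-based material and provides four stay positions, likely for occupants of the block.
; On BeginPlay it caches the world locations of its four StayLocation components in an array, disables box collision and applies the material from BlockType indexed by Type.
; SetMaterialBegin reapplies only the material, while Tick does so every frame when Change is true.
; The BlockType RepNotify is empty.
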(event `self.ReceiveTick`
  (params (DeltaSeconds :type "Float (single-precision)"))
  (if (`self.Change`)
    (`PrimitiveComponent.SetMaterial` (`self.Block`) 0 (`|GetArrayItem` (`self.BlockType`) (`self.Type`)))))

(event `self.ReceiveBeginPlay`
  (`self.F_SetStayLocation` 0 (`self.StayLocation1`))
  (`self.F_SetStayLocation` 1 (`self.StayLocation2`))
  (`self.F_SetStayLocation` 2 (`self.StayLocation3`))
  (`self.F_SetStayLocation` 3 (`self.StayLocation4`))
  (`PrimitiveComponent.SetCollisionEnabled` (`self.BoxCollision`) "NoCollision")
  (`PrimitiveComponent.SetMaterial` (`self.Block`) 0 (`|GetArrayItem` (`self.BlockType`) (`self.Type`)) :!label _label))

(event `Set Material Begin`
  (goto _label))

(fn `F_SetStayLocation`
  (params (Index :type Integer) (Target :type "SceneComponent Object Reference"))
  (`KismetArrayLibrary.Array_Set` (`self.StayLocation`) Index (`SceneComponent.K2_GetComponentLocation` Target)))

(fn `OnRep_BlockType`)

(fn `UserConstructionScript`)