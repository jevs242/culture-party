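; Obstacle course spawner that places one platform at its own location and rotation on BeginPlay.
; IntentoDeSpawnear spawns only when CurrentPlatform is invalid, then stores the new actor there.
; The class comes from PlataformaToSpawn by random index, but the maximum is the last index of a one-element array holding the length, so it always picks the first entry.
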(event `self.ReceiveBeginPlay`
  (`self.Intento de spawnear`))

(fn `Intento de spawnear`
  (`/Engine/EditorBlueprintResources/StandardMacros.IsValid` (`self.CurrentPlatform`)
    (:`Is Not Valid`
      (`self.SpawnearPlataforma`))))

(fn `SpawnearPlataforma`
  (bind _returnvalue (`|SpawnActorFromClass` (`|GetArrayItem` (`self.PlataformaToSpawn`) (`KismetMathLibrary.RandomIntegerInRange` 0 (`KismetArrayLibrary.Array_LastIndex` (`|MakeArray` (`KismetArrayLibrary.Array_Length` (`self.PlataformaToSpawn`)))))) (`KismetMathLibrary.MakeTransform` (`self.K2_GetActorLocation`) (`self.K2_GetActorRotation`)) "AdjustIfPossibleButAlwaysSpawn" "OverrideRootScale" null null))
  (set `self.CurrentPlatform` _returnvalue))

(fn `UserConstructionScript`)