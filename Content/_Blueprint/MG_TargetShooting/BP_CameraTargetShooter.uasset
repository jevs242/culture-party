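; Player pawn for the target-shooting party minigame: a camera with yaw and pitch limits by player number that fires BP_Bullet from the view, spawned on authority.
; After an intro countdown it reverses one of the player's BP_Targets, picked randomly without immediate repeats, shortening the delay between raises.
; Points accumulate in steps and feed the timer widget on authority each tick.
; When time expires it disables input and reports to the game mode.
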(event `SetPoints Client`
  (params (Points :type Integer))
  ;[1 1 1] Set Client Event
)

(event `Points W`
  (bind _w_minigames (`self.W Minigames`))
  ;[1 1 1] Set Client Event
  (`/Engine/EditorBlueprintResources/StandardMacros.IsValid` _w_minigames
    (:`Is Valid`
      (bind _outactors (`GameplayStatics.GetAllActorsOfClass` "BP_CameraTargetShooter_C"))
      (for _array_element _outactors
        (`KismetArrayLibrary.Array_Set` (`/Game/UI/Widgets/WBP_MiniGames.Points` _w_minigames) (`/Game/_Blueprint/MG_TargetShooting/BP_CameraTargetShooter.NumPlayer` _array_element) (`/Game/_Blueprint/MG_TargetShooting/BP_CameraTargetShooter.Points` _array_element))))))

(event `GameMode Server`
  ;[1 1 1] Set Server Event
  (`self.Remove Widget`)
  (`self.DisableInput` (`GameplayStatics.GetPlayerController` 0))
  (bind _asbp_capstone_game_mode_base (cast `/Game/_Blueprint/_Base/BP_CapstoneGameModeBase` (`GameplayStatics.GetGameMode`)))
  (`/Game/_Blueprint/_Base/BP_CapstoneGameModeBase.Game conclusion : Target Shooting` _asbp_capstone_game_mode_base self))

(event `self.ReceiveBeginPlay`
  (bind _returnvalue (`GameplayStatics.GetPlayerCameraManager` 0))
  (bind _returnvalue_2 (`GameplayStatics.GetPlayerController` 0))
  ;[1 1 1] Game
  (`KismetSystemLibrary.Delay` 1.0)
  (cast `/Game/_Blueprint/_Base/BP_PartyPlayerController` (`GameplayStatics.GetPlayerController` 0))
  (if (or (== (`self.NumPlayer`) 0) (== (`self.NumPlayer`) 2))
    (`self.Set View Yaw Pitch Client` 140.0 220.0 _returnvalue -40.0 40.0)
    (else
      (`self.Set View Yaw Pitch Client` -40.0 40.0 _returnvalue -40.0 40.0)))
  (if (`self.IsLocallyControlled`)
    (bind _returnvalue_3 (`|CreateWidget` "/Game/_Blueprint/MG_TargetShooting/WBP_Crosshair.WBP_Crosshair_C" (`GameplayStatics.GetPlayerController` 0)))
    (`UserWidget.AddToPlayerScreen` _returnvalue_3 0))
  (set `PlayerController.bShowMouseCursor` false _returnvalue_2)
  (if (`self.IsLocallyControlled`)
    (bind _returnvalue_4 (`|CreateWidget` "/Game/UI/Widgets/WBP_CounterMiniGames.WBP_CounterMiniGames_C" _returnvalue_2 (`KismetMathLibrary.FTrunc` (`self.TimeBegin`))))
    (`UserWidget.AddToPlayerScreen` _returnvalue_4 0)
    (`KismetSystemLibrary.Delay` (`self.TimeBegin`))
    (`self.End Game Server`)
    (`self.Up Now Server`)))

(event `InputAxis|Turn`
  (params (AxisValue :type "Float (single-precision)"))
  ;[1 1 1] Game
  (`self.AddControllerYawInput` (* AxisValue 0.5)))

(event `End Game Server`
  ;[1 1 1] Set Server Event
  (`self.Widget`)
  (`KismetSystemLibrary.Delay` (`self.TimeEnd`))
  (`self.GameMode Server`))

(event `Set View Yaw Pitch Client`
  (params (`View Yaw Min` :type "Float (double-precision)") (`View Yaw Max` :type "Float (double-precision)") (InputPin :type "PlayerCameraManager Object Reference") (`View Pitch Min` :type "Float (double-precision)") (`View Pitch Max` :type "Float (double-precision)"))
  ;[1 1 1] Set Client Event
  (`/Engine/EditorBlueprintResources/StandardMacros.IsValid` InputPin
    (:`Is Valid`
      (set `PlayerCameraManager.ViewYawMin` `View Yaw Min` InputPin)
      (set `PlayerCameraManager.ViewYawMax` `View Yaw Max` InputPin)
      (set `PlayerCameraManager.ViewPitchMin` `View Pitch Min` InputPin)
      (set `PlayerCameraManager.ViewPitchMax` `View Pitch Max` InputPin))))

(event `Widget`
  ;[1 1 1] Set Server Event
  (if (`self.IsLocallyControlled`)
    (bind _returnvalue (`|CreateWidget` "/Game/UI/Widgets/WBP_MiniGames.WBP_MiniGames_C" (`GameplayStatics.GetPlayerController` 0) (`self.TimeEnd`)))
    (bind _output_get (set `self.W Minigames` _returnvalue))
    (`UserWidget.AddToPlayerScreen` _output_get 0)))

(event `InputAxis|LookUp`
  (params (AxisValue :type "Float (single-precision)"))
  ;[1 1 1] Game
  (`self.AddControllerPitchInput` (* AxisValue 0.5)))

(event `Shoot`
  (params (Location :type "Vector Structure") (`Camara Rotator` :type "Rotator Structure"))
  ;[1 1 1] Game
  (`/Engine/EditorBlueprintResources/ActorMacros.Switch Has Authority`
    (:`Authority`
      (bind _returnvalue (`|SpawnActorFromClass` "/Game/_Blueprint/MG_TargetShooting/BP_Bullet.BP_Bullet_C" (`KismetMathLibrary.MakeTransform` Location `Camara Rotator`) "AdjustIfPossibleButAlwaysSpawn" "OverrideRootScale" null null)) ; Spawn projectile
      (set `/Game/_Blueprint/MG_TargetShooting/BP_Bullet.Character` self _returnvalue))))

(event `Random Up Server`
  ;[1 1 1] Set Server Event
  (bind _output_get (set `self.RandomUp` (`KismetMathLibrary.RandomIntegerInRange` 1 3)))
  (if (== (`self.RandomUp`) (`self.RandomPas`))
    (`self.Random Up Server`)
    (else
      (set `self.RandomPas` _output_get))))

(event `InputAction|Shoot`
  (params (Key :type "Key Structure"))
  (bind _returnvalue (`GameplayStatics.GetPlayerCameraManager` 0))
  ;[1 1 1] Game
  (:`Pressed`
    (`self.Shoot` (`PlayerCameraManager.GetCameraLocation` _returnvalue) (`PlayerCameraManager.GetCameraRotation` _returnvalue))))

(event `Remove Widget All`
  ;[1 1 1] Set Client Event
  (`WidgetLayoutLibrary.RemoveAllWidgets`))

(event `self.ReceiveTick`
  (params (DeltaSeconds :type "Float (single-precision)"))
  ;[1 1 1] Game
  (`/Engine/EditorBlueprintResources/ActorMacros.Switch Has Authority`
    (:`Authority`
      (`self.Points W`))))

(event `Up Now Server`
  ;[1 1 1] Set Server Event
  (set `self.TimeUp` (`KismetMathLibrary.FClamp` (- (`self.TimeUp`) 1.0) 0.05 5.0) :!label _label)
  (`self.Random Up Server`)
  (bind _outactors (`GameplayStatics.GetAllActorsOfClass` "/Game/_Blueprint/MG_TargetShooting/BP_Target.BP_Target_C"))
  (for _array_element _outactors
    (if (== (`/Game/_Blueprint/MG_TargetShooting/BP_Target.TagPlayer` _array_element) (`self.NumPlayer`))
      (if (== (`self.RandomUp`) (`/Game/_Blueprint/MG_TargetShooting/BP_Target.TagTarget` _array_element))
        (`/Game/_Blueprint/MG_TargetShooting/BP_Target.Reverse` _array_element)))))

(event `Remove Widget`
  ;[1 1 1] Set Client Event
  (`/Engine/EditorBlueprintResources/ActorMacros.Switch Has Authority`
    (:`Authority`
      (`self.Remove Widget All`))))

(event `Up Server Server`
  ;[1 1 1] Set Server Event
  (`KismetSystemLibrary.Delay` (`self.TimeUp`))
  (goto _label))

(event `Sum Points Server`
  ;[1 1 1] Set Server Event
  (bind _output_get (set `self.Points` (+ (`self.Points`) 10)))
  (`self.SetPoints Client` _output_get))

(fn `UserConstructionScript`)