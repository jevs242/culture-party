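; BP_Target is a shooting minigame target that falls when hit by a bullet from the player matching its TagPlayer.
; Bullet overlaps play a sound and hide the bullet; a valid hit on a standing target triggers effects, awards points on authority and starts the fall.
; A timeline rolls the Agarre component down, or back up via Reverse, which re-arms it, routing rotation and state through Server-named events.
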(event `The_Target`
  (bind _returnvalue (`self.K2_GetActorLocation`))
  (bind _character (`/Game/_Blueprint/MG_TargetShooting/BP_Bullet.Character` (`self.Ref Bala`)))
  (if (== (`/Game/_Blueprint/MG_TargetShooting/BP_CameraTargetShooter.NumPlayer` (`/Game/_Blueprint/MG_TargetShooting/BP_Bullet.Character` (`self.Ref Bala`))) (`self.TagPlayer`))
    (if (not (`self.Down?`))
      (`self.Set Down? Server` true)
      (`GameplayStatics.SpawnEmitterAtLocation` null _returnvalue)
      (`GameplayStatics.PlaySoundAtLocation` null _returnvalue (struct) 1.0 1.0 0.0 null null null)
      (`/Engine/EditorBlueprintResources/ActorMacros.Switch Has Authority`
        (:`Authority`
          (`/Game/_Blueprint/MG_TargetShooting/BP_CameraTargetShooter.Sum Points Server` _character))
        (:`Remote`
          _))
      (`/Game/_Blueprint/MG_TargetShooting/BP_CameraTargetShooter.Up Server Server` _character)
      (`self.Down`))))

(event `Set Relative Rotation Server`
  (params (`New Rotation X (Roll)` :type "Float (double-precision)") (`New Rotation Y (Pitch)` :type "Float (double-precision)") (`New Rotation Z (Yaw)` :type "Float (double-precision)"))
  (`SceneComponent.K2_SetRelativeRotation` (`self.Agarre`) (`KismetMathLibrary.MakeRotator` `New Rotation X (Roll)` `New Rotation Y (Pitch)` `New Rotation Z (Yaw)`) false false))

(event `Set Down? Server`
  (params (`Down?` :type Boolean))
  (set `self.Down?` `Down?`))

(event `Set Reverse? Server`
  (params (`Reverse?` :type Boolean))
  (set `self.Reverse?` `Reverse?`))

(event `Reverse`
  (bind (_relativerotation_roll _relativerotation_pitch _relativerotation_yaw) (`KismetMathLibrary.BreakRotator` (`SceneComponent.RelativeRotation` (`self.Agarre`))))
  (`self.Set Reverse? Server` true)
  (bind (_direction _float) (`Timeline|Timeline_0` :!via `ReverseFromEnd` :!label _label)
    (:`Update`
      (`self.Set Relative Rotation Server` _float _relativerotation_pitch _relativerotation_yaw))
    (:`Finished`
      (if (`self.Reverse?`)
        (`self.Set Down? Server` false)
        (`self.Set Reverse? Server` false)))))

(event `Down`
  (goto _label :!via `PlayFromStart`))

(event `self.TargetCollision.OnComponentBeginOverlap`
  (params (OverlappedComponent :type "PrimitiveComponent Object Reference") (OtherActor :type "Actor Object Reference") (OtherComp :type "PrimitiveComponent Object Reference") (OtherBodyIndex :type Integer) (bFromSweep :type Boolean) (SweepResult :type "HitResult Structure (by ref)"))
  (bind _asbp_bullet (cast `/Game/_Blueprint/MG_TargetShooting/BP_Bullet` OtherActor))
  (bind _output_get (set `self.Ref Bala` _asbp_bullet))
  (`GameplayStatics.PlaySound2D` "/Game/Music/TARGET_SOUND2_Cue.TARGET_SOUND2_Cue" 1.0 1.0 0.0 null null)
  (`self.SetActorHiddenInGame` _output_get true)
  (`self.The_Target`))

(fn `UserConstructionScript`)