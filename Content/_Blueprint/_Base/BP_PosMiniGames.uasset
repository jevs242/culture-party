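; BP_PosMiniGames is a mini-game positioning Blueprint that records start transforms for four player slots.
; On BeginPlay, the N_StartLocation graph calls F_SetStartLocation once for each of Player1 to Player4.
; That function writes the target's world transform into the StartLocation array at the matching zero-based index.
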(event `self.ReceiveBeginPlay`
  (`self.F_SetStartLocation` 0 (`self.Player1`))
  (`self.F_SetStartLocation` 1 (`self.Player2`))
  (`self.F_SetStartLocation` 2 (`self.Player3`))
  (`self.F_SetStartLocation` 3 (`self.Player4`)))

(fn `F_SetStartLocation`
  (params (Index :type Integer) (Target :type "SceneComponent Object Reference"))
  (`KismetArrayLibrary.Array_Set` (`self.StartLocation`) Index (`SceneComponent.K2_GetComponentToWorld` Target)))

(fn `UserConstructionScript`)