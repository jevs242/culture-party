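; BP_PartyGameInstance is a Game Instance Blueprint that handles session hosting and joining for a party game and stores a NowBlock value.
; SessionHost creates a session for the first player controller, ignoring its UseLAN input, and opens Map as a listen server on success.
; JoinSession joins a supplied search result and only prints the outcome.
; An advanced session node is left unconnected.
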(event `Set`
  (params (NowBlock :type Integer))
  (set `self.NowBlock` NowBlock))

(event `Session Host`
  (params (bUseLAN :type Boolean))
  (`CreateSessionCallbackProxy.CreateSession` (`GameplayStatics.GetPlayerController` 0)
    (:`OnSuccess`
      (`KismetSystemLibrary.PrintString` "Host Success")
      (`GameplayStatics.OpenLevel` "Map" true "listen"))
    (:`OnFailure`
      (`KismetSystemLibrary.PrintString` "Host Fail"))))

(event `Join Session`
  (params (SearchResult :type "BlueprintSessionResult Structure (by ref)"))
  (`JoinSessionCallbackProxy.JoinSession` (`GameplayStatics.GetPlayerController` 0) SearchResult
    (:`OnSuccess`
      (`KismetSystemLibrary.PrintString` "Hello"))
    (:`OnFailure`
      (`KismetSystemLibrary.PrintString` "Join Fail"))))