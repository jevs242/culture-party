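; Game mode that concludes a tap-based boat minigame and returns players to the party through the party player controller.
; Each Gameconclusion:Tap call gives the reporting BP_CamaraPlayerTap the next finishing position and stops its boat.
; The first call starts a ten-second Delay, during which others can still place.
; It then calls ReturnParty, prints each player's position and destroys the tap camera actors.
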(event `self.ReceiveBeginPlay`
  (bind _asbp_party_player_controller (cast `/Game/_Blueprint/_Base/BP_PartyPlayerController` (`GameplayStatics.GetPlayerController` 0)))
  (set `self.PlayerController` _asbp_party_player_controller))

(event `Game conclusion : Tap`
  (params (CamaraTap :type "Object Object Reference"))
  (bind _outactors (`GameplayStatics.GetAllActorsOfClass` "/Game/_Blueprint/MG_Tap/BP_CamaraPlayerTap.BP_CamaraPlayerTap_C"))
  (for _array_element _outactors
    (if (== _array_element CamaraTap)
      (bind _output_get (set `self.Pos` (+ (`self.Pos`) 1)))
      (set `/Game/_Blueprint/MG_Tap/BP_CamaraPlayerTap.Pos` _output_get _array_element)
      (set `/Game/_Blueprint/MG_Tap/BP_CamaraPlayerTap.NowMoveBoat` false _array_element)))
  (`KismetSystemLibrary.Delay` 10.0)
  (`/Game/_Blueprint/_Base/BP_PartyPlayerController.Return Party` (`self.PlayerController`))
  (for (_array_element_2 _array_index) _outactors
    (bind _result (`/Engine/EditorBlueprintResources/StandardMacros.IncrementInt` _array_index)
      (:`  `
        (`KismetSystemLibrary.PrintString` (`KismetStringLibrary.Concat_StrStr` "El  " "Jugador " (`KismetStringLibrary.Conv_IntToString` _result) " quedo " (`KismetStringLibrary.Conv_IntToString` (`/Game/_Blueprint/MG_Tap/BP_CamaraPlayerTap.Pos` _array_element_2))) true true (struct :`G` 0.66 :`B` 1.0 :`A` 1.0) 10.0)
        (`self.K2_DestroyActor` _array_element_2)))))

(fn `UserConstructionScript`)