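; Backup-named party game mode that ranks players as they finish the Tap, Bottle Flip, Target Shooting and Obstacle Course minigames.
; Tap counts positions down, Bottle Flip and Obstacle Course count up, and Target Shooting ranks scores by repeated max extraction.
; After a hard-coded two finishers, the first three call ReturnParty on the party controller and destroy their player actors.
; Obstacle Course only assigns positions; its ReturnParty call is disconnected.
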(event `self.ReceiveBeginPlay`
  (bind _asbp_party_player_controller (cast `/Game/_Blueprint/_Base/BP_PartyPlayerController` (`GameplayStatics.GetPlayerController` 0)))
  (bind _output_get (set `self.PlayerController` _asbp_party_player_controller))
  (bind _result (`/Engine/EditorBlueprintResources/StandardMacros.IncrementInt` (`KismetArrayLibrary.Array_LastIndex` (`/Game/_Blueprint/_Base/BP_PartyPlayerController.Turn` _output_get)))
    (:`  `
      (set `self.PosTap` _result))))

(event `Game conclusion : Tap`
  (params (CamaraTap :type "Object Object Reference"))
  (bind _outactors (`GameplayStatics.GetAllActorsOfClass` "/Game/_Blueprint/MG_Tap/BP_CamaraPlayerTap.BP_CamaraPlayerTap_C"))
  (for (_array_element _array_index) _outactors
    (if (== _array_element CamaraTap)
      (bind _output_get (set `self.PosTap` (- (`self.PosTap`) 1)))
      (set `/Game/_Blueprint/MG_Tap/BP_CamaraPlayerTap.Pos` _output_get _array_element)
      (set `/Game/_Blueprint/MG_Tap/BP_CamaraPlayerTap.NowMoveBoat` false _array_element)
      (set `self.CounterTap` (+ (`self.CounterTap`) 1))
      (`KismetSystemLibrary.PrintString` (`KismetStringLibrary.Concat_StrStr` "El  " "Jugador " (`KismetStringLibrary.Conv_IntToString` (+ _array_index 1)) " quedo " (`KismetStringLibrary.Conv_IntToString` (+ (`/Game/_Blueprint/MG_Tap/BP_CamaraPlayerTap.Pos` _array_element) 0))) true true (struct :`G` 0.66 :`B` 1.0 :`A` 1.0) 10.0)))
  (if (== (`self.CounterTap`) 2)
    (`KismetSystemLibrary.Delay` 10.0)
    (`/Game/_Blueprint/_Base/BP_PartyPlayerController.Return Party` (`self.PlayerController`))
    (bind _outactors_2 (`GameplayStatics.GetAllActorsOfClass` "/Game/_Blueprint/MG_Tap/BP_CamaraPlayerTap.BP_CamaraPlayerTap_C"))
    (for _array_element_2 _outactors_2
      (`self.K2_DestroyActor` _array_element_2))
    (set `self.CounterTap` 0)
    (bind _result (`/Engine/EditorBlueprintResources/StandardMacros.IncrementInt` (`KismetArrayLibrary.Array_LastIndex` (`/Game/_Blueprint/_Base/BP_PartyPlayerController.Turn` (`self.PlayerController`))))
      (:`  `
        (set `self.PosTap` _result)))))

(event `Game conclusion : Bottle Flip`
  (params (Camara :type "Object Object Reference"))
  (bind _outactors (`GameplayStatics.GetAllActorsOfClass` "/Game/_Blueprint/MG_BottleFlip/BP_CamaraBottleFlip.BP_CamaraBottleFlip_C"))
  (for _array_element _outactors
    (if (== _array_element Camara)
      (bind _output_get (set `self.PosBottleFlip` (+ (`self.PosBottleFlip`) 1)))
      (set `/Game/_Blueprint/MG_BottleFlip/BP_CamaraBottleFlip.Pos` _output_get _array_element)
      (`KismetSystemLibrary.PrintString` (`KismetStringLibrary.Concat_StrStr` "Jugador " (`KismetStringLibrary.Conv_IntToString` (+ (`/Game/_Blueprint/MG_BottleFlip/BP_CamaraBottleFlip.PlayerNum` _array_element) 1)) " quedo" (`KismetStringLibrary.Conv_IntToString` (`/Game/_Blueprint/MG_BottleFlip/BP_CamaraBottleFlip.Pos` _array_element))))))
  (if (== (`self.PosBottleFlip`) 2)
    (`/Game/_Blueprint/_Base/BP_PartyPlayerController.Return Party` (`self.PlayerController`))
    (bind _outactors_2 (`GameplayStatics.GetAllActorsOfClass` "/Game/_Blueprint/MG_BottleFlip/BP_CamaraBottleFlip.BP_CamaraBottleFlip_C"))
    (for _array_element_2 _outactors_2
      (`self.K2_DestroyActor` _array_element_2))
    (set `self.PosBottleFlip` 0)))

(event `Game conclusion : Target Shooting`
  (params (Character :type "/Game/_Blueprint/MG_Tiro_Al_Blanco/Tiro_Al_Blanco_Character Object Reference"))
  (bind _indexofmaxvalue (`KismetMathLibrary.MaxOfIntArray` (`self.Points`)))
  (bind _outactors (`GameplayStatics.GetAllActorsOfClass` "/Game/_Blueprint/MG_Tiro_Al_Blanco/Tiro_Al_Blanco_Character.Tiro_Al_Blanco_Character_C"))
  (for (_array_element _array_index) _outactors
    (if (== Character _array_element)
      (`KismetArrayLibrary.Array_Set` (`self.Points`) _array_index (`/Game/_Blueprint/MG_Tiro_Al_Blanco/Tiro_Al_Blanco_Character.Points` _array_element))
      (bind _result (`/Engine/EditorBlueprintResources/StandardMacros.IncrementInt` (`self.Counter`))
        (:`  `
          (set `self.Counter` _result)))))
  (if (== (`self.Counter`) 2)
    (for _ (range (+ (`KismetArrayLibrary.Array_LastIndex` (`self.Points`)) 1))
      (bind _outactors_2 (`GameplayStatics.GetAllActorsOfClass` "/Game/_Blueprint/MG_Tiro_Al_Blanco/Tiro_Al_Blanco_Character.Tiro_Al_Blanco_Character_C"))
      (bind _output_get (set `self.PosTargetShooting` (+ (`self.PosTargetShooting`) 1)))
      (bind _output (`|GetArrayItem` _outactors_2 _indexofmaxvalue))
      (bind _output_get_2 (set `/Game/_Blueprint/MG_Tiro_Al_Blanco/Tiro_Al_Blanco_Character.Pos` _output_get _output))
      (`KismetSystemLibrary.PrintString` (`KismetStringLibrary.Concat_StrStr` "Jugador " (`KismetStringLibrary.Conv_IntToString` (+ (`/Game/_Blueprint/MG_Tiro_Al_Blanco/Tiro_Al_Blanco_Character.NumPlayer` _output) 1)) " Quedo " (`KismetStringLibrary.Conv_IntToString` _output_get_2)) true true (struct :`G` 0.66 :`B` 1.0 :`A` 1.0) 10.0)
      (`KismetArrayLibrary.Array_Set` (`self.Points`) _indexofmaxvalue -1))
    (`/Game/_Blueprint/_Base/BP_PartyPlayerController.Return Party` (`self.PlayerController`))
    (bind _outactors_3 (`GameplayStatics.GetAllActorsOfClass` "/Game/_Blueprint/MG_Tiro_Al_Blanco/Tiro_Al_Blanco_Character.Tiro_Al_Blanco_Character_C"))
    (for _array_element_2 _outactors_3
      (`self.K2_DestroyActor` _array_element_2))
    (set `self.PosTargetShooting` 0)))

(event `GameConclusion: ObstacleCourse`
  (params (RunnerCharacter :type "/Game/_Blueprint/Obstacle_Course/RunnerCharacter Object Reference"))
  (bind _outactors (`GameplayStatics.GetAllActorsOfClass` "/Game/_Blueprint/Obstacle_Course/RunnerCharacter.RunnerCharacter_C"))
  (for _array_element _outactors
    (if (== RunnerCharacter _array_element)
      (bind _output_get (set `self.RunnerPositions` (+ (`self.RunnerPositions`) 1)))
      (set `/Game/_Blueprint/Obstacle_Course/RunnerCharacter.CharactersPositions` _output_get _array_element)
      (`KismetSystemLibrary.PrintString` (`KismetStringLibrary.Concat_StrStr` "Jugador " (`KismetStringLibrary.Conv_IntToString` (+ (`/Game/_Blueprint/Obstacle_Course/RunnerCharacter.PlayerNum` _array_element) 1)) "Quedo Posicion" (`KismetStringLibrary.Conv_IntToString` (`/Game/_Blueprint/Obstacle_Course/RunnerCharacter.CharactersPositions` _array_element))))))
  (if (== (`self.RunnerPositions`) 2)
    _))

(fn `UserConstructionScript`)