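; Game mode that ends four party minigames (Tap, Bottle Flip, Target Shooting, Obstacle Course), assigning player placements and returning to the party through the cached player controller.
; Tap and Target Shooting collect scores, then rank by repeatedly taking the array maximum.
; Bottle Flip and Obstacle Course rank by report order.
; Completion triggers at two reports; minigame actors are then destroyed, except runners, which have a separate DeleteRunning event, and Obstacle Course adds timed returns.
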(event `BeginPlay`
  (bind _outactors (`GameplayStatics.GetAllActorsOfClass` "/Game/_Blueprint/_Party/BP_CamaraPlayer.BP_CamaraPlayer_C"))
  (for _ _outactors
    (`KismetArrayLibrary.Array_Add` (`self.Tap`))
    (`KismetArrayLibrary.Array_Add` (`self.Points`))))

(event `self.ReceiveBeginPlay`
  (bind _asbp_party_player_controller (cast `/Game/_Blueprint/_Base/BP_PartyPlayerController` (`GameplayStatics.GetPlayerController` 0)))
  (set `self.PlayerController` _asbp_party_player_controller))

(event `Game conclusion : Tap`
  (params (CamaraTap :type "Object Object Reference"))
  (bind _indexofmaxvalue (`KismetMathLibrary.MaxOfIntArray` (`self.Tap`)))
  (bind _outactors (`GameplayStatics.GetAllActorsOfClass` "/Game/_Blueprint/MG_Tap/BP_CamaraPlayerTap.BP_CamaraPlayerTap_C"))
  (for (_array_element _array_index) _outactors
    (if (== _array_element CamaraTap)
      (`KismetArrayLibrary.Array_Set` (`self.Tap`) _array_index (`/Game/_Blueprint/MG_Tap/BP_CamaraPlayerTap.Tap` _array_element))
      (set `/Game/_Blueprint/MG_Tap/BP_CamaraPlayerTap.NowMoveBoat` false _array_element)
      (set `self.CounterTap` (+ (`self.CounterTap`) 1))))
  (if (== (`self.CounterTap`) 2)
    (for _ (range (+ (`KismetArrayLibrary.Array_LastIndex` (`self.Tap`)) 1))
      (bind _outactors_2 (`GameplayStatics.GetAllActorsOfClass` "/Game/_Blueprint/MG_Tap/BP_CamaraPlayerTap.BP_CamaraPlayerTap_C"))
      (bind _output_get (set `self.PosTap` (+ (`self.PosTap`) 1)))
      (bind _output (`|GetArrayItem` _outactors_2 _indexofmaxvalue))
      (set `/Game/_Blueprint/MG_Tap/BP_CamaraPlayerTap.Pos` _output_get _output)
      (`KismetSystemLibrary.PrintString` (`KismetStringLibrary.Concat_StrStr` "Jugador " (`KismetStringLibrary.Conv_IntToString` (+ (`/Game/_Blueprint/MG_Tap/BP_CamaraPlayerTap.PlayerNum` _output) 1)) " Quedo " (`KismetStringLibrary.Conv_IntToString` (`self.PosTap`))) true true (struct :`G` 0.66 :`B` 1.0 :`A` 1.0) 10.0)
      (`KismetArrayLibrary.Array_Set` (`self.Tap`) _indexofmaxvalue -1))
    (`KismetSystemLibrary.Delay` 5.0)
    (`/Game/_Blueprint/_Base/BP_PartyPlayerController.Return Party` (`self.PlayerController`))
    (bind _outactors_3 (`GameplayStatics.GetAllActorsOfClass` "/Game/_Blueprint/MG_Tap/BP_CamaraPlayerTap.BP_CamaraPlayerTap_C"))
    (for _array_element_2 _outactors_3
      (`self.K2_DestroyActor` _array_element_2))
    (set `self.CounterTap` 0)
    (set `self.PosTap` 0)))

(event `Game conclusion : Bottle Flip`
  (params (Camara :type "Object Object Reference"))
  (bind _outactors (`GameplayStatics.GetAllActorsOfClass` "/Game/_Blueprint/MG_BottleFlip/BP_CamaraBottleFlip.BP_CamaraBottleFlip_C"))
  (for _array_element _outactors
    (if (== _array_element Camara)
      (bind _output_get (set `self.PosBottleFlip` (+ (`self.PosBottleFlip`) 1)))
      (set `/Game/_Blueprint/MG_BottleFlip/BP_CamaraBottleFlip.Pos` _output_get _array_element)
      (`KismetSystemLibrary.PrintString` (`KismetStringLibrary.Concat_StrStr` "Jugador " (`KismetStringLibrary.Conv_IntToString` (+ (`/Game/_Blueprint/MG_BottleFlip/BP_CamaraBottleFlip.PlayerNum` _array_element) 1)) " quedo" (`KismetStringLibrary.Conv_IntToString` (`/Game/_Blueprint/MG_BottleFlip/BP_CamaraBottleFlip.Pos` _array_element))))))
  (if (== (`self.PosBottleFlip`) 2)
    (`/Game/_Blueprint/_Base/BP_PartyPlayerController.Return Party` (`self.PlayerController`))
    (bind _outactors_2 (`GameplayStatics.GetAllActorsOfClass` "/Game/_Blueprint/MG_BottleFlip/BP_CamaraBottleFlip.BP_CamaraBottleFlip_C"))
    (for _array_element_2 _outactors_2
      (`self.K2_DestroyActor` _array_element_2))
    (set `self.PosBottleFlip` 0)))

(event `Game conclusion : Target Shooting`
  (params (Character :type "/Game/_Blueprint/MG_Tiro_Al_Blanco/BP_CharacterTargetShooter Object Reference"))
  (bind _indexofmaxvalue (`KismetMathLibrary.MaxOfIntArray` (`self.Points`)))
  (bind _outactors (`GameplayStatics.GetAllActorsOfClass` "/Game/_Blueprint/MG_Tiro_Al_Blanco/BP_CharacterTargetShooter.BP_CharacterTargetShooter_C"))
  (for (_array_element _array_index) _outactors
    (if (== Character _array_element)
      (`KismetArrayLibrary.Array_Set` (`self.Points`) _array_index (`/Game/_Blueprint/MG_Tiro_Al_Blanco/BP_CharacterTargetShooter.Points` _array_element))
      (bind _result (`/Engine/EditorBlueprintResources/StandardMacros.IncrementInt` (`self.CounterTargetShooting`))
        (:`  `
          (set `self.CounterTargetShooting` _result)))))
  (if (== (`self.CounterTargetShooting`) 2)
    (for _ (range (+ (`KismetArrayLibrary.Array_LastIndex` (`self.Points`)) 1))
      (bind _outactors_2 (`GameplayStatics.GetAllActorsOfClass` "/Game/_Blueprint/MG_Tiro_Al_Blanco/BP_CharacterTargetShooter.BP_CharacterTargetShooter_C"))
      (bind _output_get (set `self.PosTargetShooting` (+ (`self.PosTargetShooting`) 1)))
      (bind _output (`|GetArrayItem` _outactors_2 _indexofmaxvalue))
      (bind _output_get_2 (set `/Game/_Blueprint/MG_Tiro_Al_Blanco/BP_CharacterTargetShooter.Pos` _output_get _output))
      (`KismetSystemLibrary.PrintString` (`KismetStringLibrary.Concat_StrStr` "Jugador " (`KismetStringLibrary.Conv_IntToString` (+ (`/Game/_Blueprint/MG_Tiro_Al_Blanco/BP_CharacterTargetShooter.NumPlayer` _output) 1)) " Quedo " (`KismetStringLibrary.Conv_IntToString` _output_get_2)) true true (struct :`G` 0.66 :`B` 1.0 :`A` 1.0) 10.0)
      (`KismetArrayLibrary.Array_Set` (`self.Points`) _indexofmaxvalue -1))
    (`/Game/_Blueprint/_Base/BP_PartyPlayerController.Return Party` (`self.PlayerController`))
    (bind _outactors_3 (`GameplayStatics.GetAllActorsOfClass` "/Game/_Blueprint/MG_Tiro_Al_Blanco/BP_CharacterTargetShooter.BP_CharacterTargetShooter_C"))
    (for _array_element_2 _outactors_3
      (`self.K2_DestroyActor` _array_element_2))
    (set `self.PosTargetShooting` 0)
    (set `self.CounterTargetShooting` 0)))

(event `GameConclusion: ObstacleCourse`
  (params (RunnerCharacter :type "/Game/_Blueprint/Obstacle_Course/RunnerCharacter Object Reference") (CantidadPlayers :type Integer))
  (set `self.Cantidad Players` CantidadPlayers)
  (bind _outactors (`GameplayStatics.GetAllActorsOfClass` "/Game/_Blueprint/Obstacle_Course/RunnerCharacter.RunnerCharacter_C"))
  (for _array_element _outactors
    (if (== RunnerCharacter _array_element)
      (bind _output_get (set `self.RunnerPositions` (+ (`self.RunnerPositions`) 1)))
      (set `/Game/_Blueprint/Obstacle_Course/RunnerCharacter.CharactersPositions` _output_get _array_element)
      (`KismetSystemLibrary.PrintString` (`KismetStringLibrary.Concat_StrStr` "Jugador " (`KismetStringLibrary.Conv_IntToString` (+ (`/Game/_Blueprint/Obstacle_Course/RunnerCharacter.PlayerNum` _array_element) 1)) "Quedo Posicion" (`KismetStringLibrary.Conv_IntToString` (`/Game/_Blueprint/Obstacle_Course/RunnerCharacter.CharactersPositions` _array_element))))))
  (if (== (`self.RunnerPositions`) 2)
    (`self.Terminar Partida`)
    (else
      (`KismetSystemLibrary.Delay` 120.0)
      (`/Game/_Blueprint/_Base/BP_PartyPlayerController.Return Party` (`self.PlayerController`)))))

(event `Terminar Partida`
  (if (== (`self.Cantidad Players`) 2)
    (`KismetSystemLibrary.Delay` 5.0)
    (`/Game/_Blueprint/_Base/BP_PartyPlayerController.Return Party` (`self.PlayerController`))
    (else
      (`KismetSystemLibrary.Delay` 30.0)
      (`/Game/_Blueprint/_Base/BP_PartyPlayerController.Return Party` (`self.PlayerController`)))))

(event `Delete Running`
  (bind _outactors (`GameplayStatics.GetAllActorsOfClass` "/Game/_Blueprint/Obstacle_Course/RunnerCharacter.RunnerCharacter_C"))
  (for _array_element _outactors
    (`self.K2_DestroyActor` _array_element))
  (set `self.RunnerPositions` 0))

(fn `UserConstructionScript`)