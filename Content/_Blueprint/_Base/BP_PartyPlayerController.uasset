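; Player controller for the party mode, running the board's turn and round loop and switching players into and out of minigames.
; The server shuffles turn order, picks a random non-repeating minigame after each round, swaps streamed levels and possesses each controller into that game's pawn.
; Afterwards it shows results and restores board cameras; final standings rank trophies over coins.
; Shared state is copied by looping over every party controller.
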(event `Player Num`
  ;[1 1 1] Modo : Party
  (bind _outactors (`GameplayStatics.GetAllActorsOfClass` "BP_PartyPlayerController_C"))
  (for (_ _array_index) _outactors
    _)
  (set `self.PlayerNum` _array_index))

(event `Widget`
  ;[1 1 1] Modo : Party
  (if (`self.End`)
    (bind _outactors (`GameplayStatics.GetAllActorsOfClass` "BP_PartyPlayerController_C"))
    (for _array_element _outactors
      (bind _playernum (`/Game/_Blueprint/_Base/BP_PartyPlayerController.PlayerNum` _array_element))
      (bind _trophy (`/Game/_Blueprint/_Base/BP_PartyPlayerController.Trophy` _array_element))
      (`KismetArrayLibrary.Array_Set` (`self.TrophyArray`) _playernum _trophy true)
      (bind _coins (`/Game/_Blueprint/_Base/BP_PartyPlayerController.Coins` _array_element))
      (`KismetArrayLibrary.Array_Set` (`self.CoinsArray`) _playernum _coins true)
      (`KismetArrayLibrary.Array_Set` (`self.AllPointsArray`) _playernum (+ (* _trophy 1000) _coins) true))
    (`GameplayStatics.GetAllActorsOfClass` "/Game/_Blueprint/_Party/BP_CharacterPlayer.BP_CharacterPlayer_C")
    (for _ (range 2)
      (bind _outactors_2 (`GameplayStatics.GetAllActorsOfClass` "BP_PartyPlayerController_C"))
      (bind _output_get (set `self.PosInt` (+ (`self.PosInt`) 1)))
      (bind _playernum_2 (`/Game/_Blueprint/_Base/BP_PartyPlayerController.PlayerNum` (`|GetArrayItem` _outactors_2 (`KismetMathLibrary.MaxOfIntArray` (`self.AllPointsArray`)))))
      (`KismetArrayLibrary.Array_Set` (`self.PosEndArray`) _playernum_2 _output_get true)
      (`KismetArrayLibrary.Array_Set` (`self.AllPointsArray`) _playernum_2 -1 true))
    (`self.Widget Outro`)))

(event `Widget Outro`
  ;[1 1 1] Modo : Party
  (if (`Pawn.IsLocallyControlled` (`GameplayStatics.GetPlayerPawn` 0))
    (bind _returnvalue (`|CreateWidget` "/Game/UI/Widgets/WBP_OutroGame.WBP_OutroGame_C" (`GameplayStatics.GetPlayerController` 0) (`self.PosEndArray`) (`self.CoinsArray`) (`self.TrophyArray`)))
    (`UserWidget.AddToPlayerScreen` _returnvalue 0)
    (set `self.End` false)))

(event `self.ReceiveBeginPlay`
  ;[1 1 1] Modo : Party
  (`KismetSystemLibrary.K2_SetTimerDelegate` (delegate `Widget`) 5.0 true)
  (`/Engine/EditorBlueprintResources/ActorMacros.Switch Has Authority`
    (:`Authority`
      (`self.Player Num`))
    (:`Remote`
      _))
  (bind _asbp_camara_player (cast `/Game/_Blueprint/_Party/BP_CamaraPlayer` (`GameplayStatics.GetPlayerPawn` 0)))
  (set `self.Ref CamaraPlayer` _asbp_camara_player)
  (`KismetSystemLibrary.Delay` 2.0)
  (`/Engine/EditorBlueprintResources/ActorMacros.Switch Has Authority`
    (:`Authority`
      (`self.Define Turn`))))

(event `ChangeToMiniGames`
  (bind _minigames (`self.MiniGames`))
  (bind _minigames_2 (`self.MiniGames`))
  ;[1 1 1] Change
  (bind _outactors (`GameplayStatics.GetAllActorsOfClass` "BP_PartyPlayerController_C"))
  (for _array_element _outactors
    (`self.Intro` _array_element _minigames_2 (`|GetArrayItem` (`self.NameMinigames`) _minigames_2)))
  (`KismetSystemLibrary.Delay` 10.0)
  (`GameplayStatics.UnloadStreamLevel` "MusicTable")
  (`GameplayStatics.LoadStreamLevel` (`|GetArrayItem` (`self.LevelName`) (`self.MiniGames`)) true)
  (bind _outactors_2 (`GameplayStatics.GetAllActorsOfClass` "BP_PartyPlayerController_C"))
  (for (_array_element_2 _array_index) _outactors_2
    (bind _outactors_3 (`GameplayStatics.GetAllActorsOfClass` "/Game/_Blueprint/_Base/BP_PosMiniGames.BP_PosMiniGames_C"))
    (for _array_element_3 _outactors_3
      (`self.Remove Widget` _array_element_2)
      (if (`KismetStringLibrary.EqualEqual_StrStr` (`/Game/_Blueprint/_Base/BP_PosMiniGames.Tag` _array_element_3) (`KismetStringLibrary.Conv_IntToString` _minigames))
        (switch `int` _minigames
          (:`0`
            (bind _output (`|GetArrayItem` (`/Game/_Blueprint/_Base/BP_PosMiniGames.StartLocation` _array_element_3) _array_index))
            (bind _returnvalue (`|SpawnActorFromClass` "/Game/_Blueprint/MG_Tap/BP_CamaraPlayerTap.BP_CamaraPlayerTap_C" _output "Undefined" "OverrideRootScale" null null))
            (`self.Possess` _array_element_2 _returnvalue))
          (:`1`
            (bind _returnvalue_2 (`|SpawnActorFromClass` "/Game/_Blueprint/MG_BottleFlip/BP_CamaraBottleFlip.BP_CamaraBottleFlip_C" _output "AlwaysSpawn" "OverrideRootScale" null null))
            (`self.Possess` _array_element_2 _returnvalue_2)
            (bind _playernum (`/Game/_Blueprint/_Base/BP_PartyPlayerController.PlayerNum` _array_element_2))
            (`/Game/_Blueprint/MG_BottleFlip/BP_CamaraBottleFlip.SetPlayerNum` _returnvalue_2 _playernum))
          (:`2`
            (bind _returnvalue_3 (`|SpawnActorFromClass` "/Game/_Blueprint/MG_Tiro_Al_Blanco/BP_CharacterTargetShooter.BP_CharacterTargetShooter_C" _output "Undefined" "OverrideRootScale" null null))
            (`self.Possess` _array_element_2 _returnvalue_3)
            (`KismetSystemLibrary.Delay` 0.2)
            (`self.Set NumPlayer` _array_element_2 _playernum _returnvalue_3))
          (:`3`
            (bind _returnvalue_4 (`|SpawnActorFromClass` "/Game/_Blueprint/Obstacle_Course/RunnerCharacter.RunnerCharacter_C" _output "Undefined" "OverrideRootScale" null null))
            (`self.Possess` _array_element_2 _returnvalue_4)
            (`/Game/_Blueprint/Obstacle_Course/RunnerCharacter.SetPlayerNum` _returnvalue_4 _playernum)))))))

(event `Set NumPlayer`
  (params (NumPlayer :type Integer) (Target :type "/Game/_Blueprint/MG_Tiro_Al_Blanco/BP_CharacterTargetShooter Object Reference"))
  ;[1 1 1] Change
  (set `/Game/_Blueprint/MG_Tiro_Al_Blanco/BP_CharacterTargetShooter.NumPlayer` NumPlayer Target))

(event `Intro`
  (params (Minigames :type Integer) (NameMinigames :type Text))
  ;[1 1 1] Change
  (bind _returnvalue (`|CreateWidget` "/Game/UI/Widgets/WBP_IntroMinigames.WBP_IntroMinigames_C" (`GameplayStatics.GetPlayerController` 0) Minigames NameMinigames))
  (`UserWidget.AddToPlayerScreen` _returnvalue 0))

(event `Define Turn`
  ;[1 1 1] Modo : Party
  (`KismetArrayLibrary.Array_Shuffle` (`self.Turn`))
  (bind _outactors (`GameplayStatics.GetAllActorsOfClass` "BP_PartyPlayerController_C"))
  (for (_ _array_index) _outactors
    (if (!= _array_index 0)
      (set `self.Turn` (`/Game/_Blueprint/_Base/BP_PartyPlayerController.Turn` (`|GetArrayItem` _outactors))))))

(event `Next Turn Server`
  ;[1 1 1] Modo : Party
  (if (<= (`self.CurrentTurn`) (`KismetArrayLibrary.Array_LastIndex` (`self.Turn`)))
    (bind _outactors (`GameplayStatics.GetAllActorsOfClass` "BP_PartyPlayerController_C"))
    (for _array_element _outactors
      (bind _output_get (set `/Game/_Blueprint/_Base/BP_PartyPlayerController.CurrentTurn` (+ (`/Game/_Blueprint/_Base/BP_PartyPlayerController.CurrentTurn` _array_element) 1) _array_element))
      (set `/Game/_Blueprint/_Base/BP_PartyPlayerController.WidgetCurrentTurn` (+ _output_get 1) _array_element))
    (`self.EndRound`)))

(event `Return Party`
  (bind _pos (`self.Pos`))
  ;[1 1 1] Modo : Return
  (`/Engine/EditorBlueprintResources/ActorMacros.Switch Has Authority`
    (:`Authority`
      (bind _outactors (`GameplayStatics.GetAllActorsOfClass` "BP_PartyPlayerController_C"))
      (for _array_element _outactors
        (set `/Game/_Blueprint/_Base/BP_PartyPlayerController.Pos` _pos _array_element)
        (`self.WBP Outro` _array_element _pos)))
    (:`Remote`
      _))
  (`KismetSystemLibrary.Delay` 10.0)
  (`/Engine/EditorBlueprintResources/ActorMacros.Switch Has Authority`
    (:`Authority`
      (`self.Return Party Server`))))

(event `WBP Outro`
  (params (POS :type "Array of Integer (by ref)"))
  ;[1 1 1] Modo : Return
  (bind _returnvalue (`|CreateWidget` "/Game/UI/Widgets/WBP_OutroMinigames.WBP_OutroMinigames_C" (`GameplayStatics.GetPlayerController` 0) POS))
  (`UserWidget.AddToPlayerScreen` _returnvalue 0))

(event `EndRound`
  ;[1 1 1] Modo : Party
  (if (== (`self.CurrentTurn`) (+ (`KismetArrayLibrary.Array_LastIndex` (`self.Turn`)) 1))
    (if (== (`self.CurrentRound`) (`self.MaxRound`))
      (bind _outactors (`GameplayStatics.GetAllActorsOfClass` "BP_PartyPlayerController_C"))
      (for _array_element _outactors
        (set `/Game/_Blueprint/_Base/BP_PartyPlayerController.End` true _array_element))
      (else
        (`KismetSystemLibrary.Delay` 1.0)
        (`self.UnPossess` (`GameplayStatics.GetPlayerController` 0))
        (`/Engine/EditorBlueprintResources/ActorMacros.Switch Has Authority`
          (:`Authority`
            (`self.Set Minijuego`)
            (bind _outactors_2 (`GameplayStatics.GetAllActorsOfClass` "BP_PartyPlayerController_C"))
            (for _array_element_2 _outactors_2
              (set `/Game/_Blueprint/_Base/BP_PartyPlayerController.MiniGames` (`self.MiniGames`) _array_element_2))
            (set `self.MiniGamesA` (`self.MiniGames`))
            (`self.ChangeToMiniGames`))
          (:`Remote`
            _))
        (bind _outactors_3 (`GameplayStatics.GetAllActorsOfClass` "/Game/_Blueprint/_Party/BP_CamaraPlayer.BP_CamaraPlayer_C"))
        (for _array_element_3 _outactors_3
          (`self.K2_DestroyActor` _array_element_3))))))

(event `Set Minijuego`
  ;[1 1 1] Modo : Party
  (set `self.MiniGames` (`KismetMathLibrary.RandomIntegerInRange` 0 3))
  (if (== (`self.MiniGames`) (`self.MiniGamesA`))
    (`self.Set Minijuego`)))

(event `Return Party Server`
  ;[1 1 1] Modo : Return
  (`GameplayStatics.LoadStreamLevel` "MusicTable" true)
  (`GameplayStatics.LoadStreamLevel` "TablaPrincipal1" true)
  (`GameplayStatics.UnloadStreamLevel` "Tap-Game")
  (`GameplayStatics.UnloadStreamLevel` "Bottle-Flip")
  (`GameplayStatics.UnloadStreamLevel` "Tiro-Al-Blanco")
  (`GameplayStatics.UnloadStreamLevel` "Carrera-De-Obstaculos")
  (bind _outactors (`GameplayStatics.GetAllActorsOfClass` "BP_PartyPlayerController_C"))
  (for (_array_element _array_index) _outactors
    (bind _outactors_2 (`GameplayStatics.GetAllActorsOfClass` "/Game/_Blueprint/_Party/BP_CharacterPlayer.BP_CharacterPlayer_C"))
    (for _array_element_2 _outactors_2
      (if (== _array_index (`/Game/_Blueprint/_Party/BP_CharacterPlayer.Tag` _array_element_2))
        (`SceneComponent.K2_SetRelativeRotation` (`Character.Mesh` _array_element_2) (`/Game/_Blueprint/_Party/BP_CharacterPlayer.BeginRotation` _array_element_2) false false)))
    (set `/Game/_Blueprint/_Base/BP_PartyPlayerController.CurrentTurn` 0 _array_element)
    (set `/Game/_Blueprint/_Base/BP_PartyPlayerController.WidgetCurrentTurn` 1 _array_element)
    (set `/Game/_Blueprint/_Base/BP_PartyPlayerController.CurrentRound` (+ (`/Game/_Blueprint/_Base/BP_PartyPlayerController.CurrentRound` _array_element) 1) _array_element)
    (`self.UnPossess` _array_element)
    (`self.UnPossess` _array_element)
    (bind _returnvalue (`|SpawnActorFromClass` "/Game/_Blueprint/_Party/BP_CamaraPlayer.BP_CamaraPlayer_C" (`KismetMathLibrary.MakeTransform` (0.0 0.0 0.0)) "Undefined" "OverrideRootScale" null null))
    (`self.Remove Widget` _array_element)
    (`self.Possess` _array_element _returnvalue)
    (`KismetSystemLibrary.Delay` 0.1)
    (`/Game/_Blueprint/_Party/BP_CamaraPlayer.Set Num Player` _returnvalue (`/Game/_Blueprint/_Base/BP_PartyPlayerController.PlayerNum` _array_element))))

(event `BeginPlay`
  (if (`self.Begin`)
    (if (== (`self.PlayerNum`) 0)
      (bind _asbp_capstone_game_mode_base (cast `/Game/_Blueprint/_Base/BP_CapstoneGameModeBase` (`GameplayStatics.GetGameMode`)))
      (`/Game/_Blueprint/_Base/BP_CapstoneGameModeBase.BeginPlay` _asbp_capstone_game_mode_base)
      (bind _outactors (`GameplayStatics.GetAllActorsOfClass` "/Game/_Blueprint/_Party/BP_CamaraPlayer.BP_CamaraPlayer_C"))
      (for (_ _array_index) _outactors
        (`KismetArrayLibrary.Array_Add` (`self.Turn`) _array_index))
      (`self.Define Turn`)
      (bind _outactors_2 (`GameplayStatics.GetAllActorsOfClass` "BP_PartyPlayerController_C"))
      (for _array_element _outactors_2
        (set `/Game/_Blueprint/_Base/BP_PartyPlayerController.Turn` (`self.Turn`) _array_element)
        (set `/Game/_Blueprint/_Base/BP_PartyPlayerController.Begin` false _array_element)))))

(event `Remove Widget`
  (`/Engine/EditorBlueprintResources/ActorMacros.Switch Has Authority`
    (:`Authority`
      (`self.Remove Widget All`))))

(event `Remove Widget All`
  (`WidgetLayoutLibrary.RemoveAllWidgets`)
  (`WidgetBlueprintLibrary.SetInputMode_GameOnly` self))

(event `PlayerReady`
  (bind _asbp_capstone_game_mode_base (cast `/Game/_Blueprint/_Base/BP_CapstoneGameModeBase` (`GameplayStatics.GetGameMode`)))
  (bind _output_get (set `/Game/_Blueprint/_Base/BP_CapstoneGameModeBase.PlayerReady` (+ (`/Game/_Blueprint/_Base/BP_CapstoneGameModeBase.PlayerReady` _asbp_capstone_game_mode_base) 1) _asbp_capstone_game_mode_base))
  (`self.Ready Server` _output_get))

(event `PlayerNoReady`
  (bind _asbp_capstone_game_mode_base (cast `/Game/_Blueprint/_Base/BP_CapstoneGameModeBase` (`GameplayStatics.GetGameMode`)))
  (bind _output_get (set `/Game/_Blueprint/_Base/BP_CapstoneGameModeBase.PlayerReady` (`KismetMathLibrary.Clamp` (- (`/Game/_Blueprint/_Base/BP_CapstoneGameModeBase.PlayerReady` _asbp_capstone_game_mode_base) 1) 0 4) _asbp_capstone_game_mode_base))
  (`self.Ready Server` _output_get))

(event `Ready Server`
  (params (PlayerReady :type Integer))
  (bind _outactors (`GameplayStatics.GetAllActorsOfClass` "BP_PartyPlayerController_C"))
  (for _array_element _outactors
    (set `/Game/_Blueprint/_Base/BP_PartyPlayerController.ReadyPlayer` PlayerReady _array_element)))

(event `Add Name`
  (params (Name :type Text))
  (set `self.Name` Name))

(event `Set Varible Server`
  (params (NowBlock :type Integer) (Coins :type Integer) (Health :type Integer) (Trophy :type Integer))
  (set `self.NowBlock` NowBlock)
  (set `self.Coins` Coins)
  (set `self.Health` Health)
  (set `self.Trophy` Trophy))

(event `PosController`
  (params (Pos :type Integer) (PNum :type Integer))
  (bind _outactors (`GameplayStatics.GetAllActorsOfClass` "BP_PartyPlayerController_C"))
  (for _array_element _outactors
    (bind _playernum (`/Game/_Blueprint/_Base/BP_PartyPlayerController.PlayerNum` _array_element))
    (if (== _playernum PNum)
      (`KismetArrayLibrary.Array_Set` (`self.Pos`) _playernum Pos))))

(fn `OnRep_TrophyArray`)

(fn `UserConstructionScript`)